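; Networked bullet actor that damages living pawns of a configured enemy class.
; On the authority, Tick destroys it once it leaves a fixed X/Y play area.
; Box overlap, also authority-only, filters for a living BP_BasePawn matching EnemyClass, applies damage credited to the instigator, fires a multicast and destroys the bullet.
; The multicast destroy event plays a 2D hit sound only where the bullet lacks authority.
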(event OnComponentBeginOverlap(Box)
  (params (OverlappedComponent :type Primitive%20Component%20Object%20Reference) (OtherActor :type Actor%20Object%20Reference) (OtherComp :type Primitive%20Component%20Object%20Reference) (OtherBodyIndex :type Integer) (bFromSweep :type Boolean) (SweepResult :type Hit%20Result%20Structure%20%28by%20ref%29))
  (Networking|SwitchHasAuthority
    (:Authority
      (bind _asbp_base_pawn (Utilities|Casting|CastToBP_BasePawn OtherActor))
      (bind _bisalive (Default|IsAlive _asbp_base_pawn))
      (if _bisalive
        (bind _enemyclass (Variables|Default|GetEnemyClass)
          (:then
            (Class|KismetSystemLibrary|IsObjectOfSoftClass OtherActor _enemyclass
              (:True
                (Game|Damage|ApplyDamage OtherActor (Variables|Default|GetDamage) (Game|GetInstigatorController) self)
                (CallFunction|MulticastonDestory)
                (Actor|DestroyActor))))
          (:else))))))

(event Custom|Multicast_OnDestory
  (Networking|SwitchHasAuthority
    (:Remote
      (Audio|PlaySound2D "/Game/Assets/Sounds/Effect2.Effect2" 1.0 1.0 0.0 0 0))))

(event EventTick
  (params (DeltaSeconds :type Float%20%28single-precision%29))
  (bind _returnvalue (Transformation|GetActorLocation))
  (Networking|SwitchHasAuthority
    (:Authority
      (if (not (and (Math|Float|InRange(Float) (.x _returnvalue) -2e+03 2e+03) (Math|Float|InRange(Float) (.y _returnvalue) -1.5e+03 1.5e+03)))
        (Actor|DestroyActor)))))

(fn ConstructionScript)