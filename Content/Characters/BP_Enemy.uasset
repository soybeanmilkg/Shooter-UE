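; BP_Enemy is an enemy character that flies or walks along negative world X while firing, then removes itself when it leaves the play area.
; On the server, Tick moves it and calls ServerShootBullet while it is alive, and destroys it outside fixed X/Y bounds.
; Its server death handler extends the parent's and has a random 50% chance to spawn a life pickup.
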(event EventServeronDie
  (|CallParentFunction)
  (if (Math|Random|RandomBool)
    (Game|SpawnActorfromClass "/Game/Pickups/BP_Pickup_Life.BP_Pickup_Life_C" (Transformation|GetActorTransform) "Undefined" "MultiplyWithRoot" 0 0)))

(event EventTick
  (params (DeltaSeconds :type Float%20%28single-precision%29))
  (bind _returnvalue (Transformation|GetActorLocation))
  (|CallParentFunction DeltaSeconds)
  (Networking|SwitchHasAuthority
    (:Authority
      (Utilities|FlowControl|Sequence
        (:then_0
          (bind _bisalive (CallFunction|IsAlive))
          (if _bisalive
            (Pawn|Input|AddMovementInput "-1.000000,0.000000,0.000000" 1.0 false)
            (CallFunction|ServerShootBullet "0, 0, 0")))
        (:then_1
          (if (not (and (Math|Float|InRange(Float) (.x _returnvalue) -2e+03 2.5e+03) (Math|Float|InRange(Float) (.y _returnvalue) -1.5e+03 1.5e+03)))
            (Actor|DestroyActor)))))))

(fn ConstructionScript
  (|CallParentFunction))