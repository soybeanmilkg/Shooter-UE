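; Player controller that routes input to BP_Player and handles the end of a run when the player dies.
; On possess it caches the pawn, then forwards Enhanced Input move and shoot actions to it.
; Unpossess is treated as death: authority stops enemy spawning and records the score in BP_GameState, while the local controller opens WBP_GameOver.
; A debug key requests the server to stop spawning; death handling does not yet account for multiplayer.
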(event Custom|Server_StopSpawnEnemy
  ;[0.15 0.003553 0.09065 0.5] 调式
  (bind _asbp_game_mode (Utilities|Casting|CastToBP_GameMode (Game|GetGameMode)))
  (Variables|/Game/GameModes/Game/BP_GameMode.BP_GameMode_C|SetbSpawnEnemies _asbp_game_mode false))

(event Input|EnhancedActionEvents|EnhancedInputActionIA_Move
  (params (ActionValue :type Vector%202D%20Structure) (ElapsedSeconds :type Float%20%28double-precision%29) (TriggeredSeconds :type Float%20%28double-precision%29) (InputAction :type Input%20Action%20Object%20Reference :default "/Game/Input/IA_Move.IA_Move"))
  ;[0.1 0.5 0.1 0.5] 输入处理
  (bind _asplayer (Variables|Default|GetAsPlayer)
    (:then
      (Class|SPlayer|Move _asplayer (.x ActionValue) (.y ActionValue)))
    (:else)))

(event Input|EnhancedActionEvents|EnhancedInputActionIA_Shoot
  (params (ActionValue :type Boolean) (ElapsedSeconds :type Float%20%28double-precision%29) (TriggeredSeconds :type Float%20%28double-precision%29) (InputAction :type Input%20Action%20Object%20Reference :default "/Game/Input/IA_Shoot.IA_Shoot"))
  ;[0.1 0.5 0.1 0.5] 输入处理
  (if ActionValue
    (bind _asplayer (Variables|Default|GetAsPlayer)
      (:then
        (Class|SPawn|ShootBullet _asplayer (Math|Vector|MakeVectorNetQuantize 0.0 0.0 0.0)))
      (:else))))

(event EventPossess
  (params (PossessedPawn :type Pawn%20Object%20Reference))
  (bind _asbp_player (Utilities|Casting|CastToBP_Player PossessedPawn))
  (Variables|Default|SetAsPlayer _asbp_player))

(event EventUnPossess
  (params (UnpossessedPawn :type Pawn%20Object%20Reference))
  ;[0.15 0.0915 0 0.5] 玩家死亡后的处理（暂时没有考虑多人游戏的情况，后面改）
  (Utilities|FlowControl|Sequence
    (:then_0
      (Networking|SwitchHasAuthority
        (:Authority
          (bind _asbp_game_mode (Utilities|Casting|CastToBP_GameMode (Game|GetGameMode)))
          (Variables|/Game/GameModes/Game/BP_GameMode.BP_GameMode_C|SetbSpawnEnemies _asbp_game_mode false)
          (bind _asbp_game_state (Utilities|Casting|CastToBP_GameState (Game|GetGameState)))
          (Class|SGameStateBase|RecordScoreInfo _asbp_game_state self))))
    (:then_1
      (if (Pawn|IsLocalController)
        (Class|SPlayerController|Goto "/Game/UI/Game/WBP_GameOver.WBP_GameOver_C")))))

(event Input|KeyboardEvents|1
  (params (Key :type Key%20Structure :default "None"))
  ;[0.15 0.003553 0.09065 0.5] 调式
  (:Pressed
    (CallFunction|ServerStopSpawnEnemy)))

(fn ConstructionScript)