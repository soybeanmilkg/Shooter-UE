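; Game mode that continuously spawns enemies during play.
; BeginPlay enables spawning after a short delay, which is skipped when the options string contains "standalone".
; Tick runs a countdown that resets to SpawnTime, each time spawning a random class from EnemyClasses at a fixed X position with a random Y offset.
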(event EventBeginPlay
  (if (Class|GameplayStatics|HasOption (Variables|Default|GetOptionsString) "standalone")
    _
    (else
      (Utilities|FlowControl|Delay 5.0)))
  (Variables|Default|SetbSpawnEnemies true))

(event EventTick
  (params (DeltaSeconds :type Float%20%28single-precision%29))
  (if (Variables|Default|GetbSpawnEnemies)
    (if (<= (Variables|Default|GetSpawnTimer) 0.0)
      (Variables|Default|SetSpawnTimer (Variables|Default|GetSpawnTime))
      (Game|SpawnActorfromClass (.OutItem (Utilities|Array|Random (Variables|Default|GetEnemyClasses))) (Math|Transform|MakeTransform (Math|Vector|MakeVector 2e+03 (Math|Random|RandomFloatinRange -1.1e+03 1.1e+03) 0.0)) "Undefined" "MultiplyWithRoot" 0 0)
      (else
        (Variables|Default|SetSpawnTimer (- (Variables|Default|GetSpawnTimer) DeltaSeconds))))))

(fn ConstructionScript)