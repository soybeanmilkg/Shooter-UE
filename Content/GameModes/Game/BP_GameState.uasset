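; BP_GameState is the game state Blueprint that relays match control requests to BP_GameMode and handles game start and end events.
; It caches the game mode on BeginPlay, runs a CommonSessionSubsystem session-owner check before start and restart, and forwards return-to-menu unchecked.
; At game end it walks PlayerArray, recording score info and notifying each BP_PlayerController.
; Start and end also print debug messages.
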(event Custom|OnGameStart
  (Development|PrintString "Game Start !!!!!!"))

(event Custom|OnGameEnd
  (for _array_element (Variables|Default|GetPlayerArray)
    (bind _asbp_player_controller (Utilities|Casting|CastToBP_PlayerController (Game|GetPlayerController _array_element)))
    (Class|SGameStateBase|RecordScoreInfo _asbp_player_controller)
    (Default|OnGameEnd _asbp_player_controller))
  (Development|PrintString "Game End !!!!!!"))

(event Custom|Start%20Game
  (params (Player :type Player%20Controller%20Object%20Reference))
  (Utilities|IsSessionOwner Player)
  (Class|GameMode|StartMatch (Variables|Default|GetAs%20BP%20Game%20Mode)))

(event Custom|Restart%20Game
  (params (Player :type Player%20Controller%20Object%20Reference))
  (Utilities|IsSessionOwner Player)
  (Class|GameMode|RestartGame (Variables|Default|GetAs%20BP%20Game%20Mode)))

(event Custom|ReturnToMainMenu
  (Class|GameModeBase|ReturntoMainMenuHost (Variables|Default|GetAs%20BP%20Game%20Mode)))

(event EventBeginPlay
  (bind _asbp_game_mode (Utilities|Casting|CastToBP_GameMode (Game|GetGameMode)))
  (Variables|Default|SetAs%20BP%20Game%20Mode _asbp_game_mode))

(fn ConstructionScript)