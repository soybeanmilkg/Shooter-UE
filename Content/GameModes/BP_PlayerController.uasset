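; Multiplayer player controller that sets up input, camera and game UI for BP_Player.
; On begin play the local controller adds the input mapping and views through the level's BP_CameraActor.
; Possession caches the pawn and, after a short delay, calls a client event that creates WBP_Game.
; Move and shoot input forward to the pawn, with shooting via a server call, and key 1 asks the server's GameMode to stop spawning enemies.
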(event Custom|Server_StopSpawnEnemy
  (bind _asbp_game_mode (Utilities|Casting|CastToBP_GameMode (Game|GetGameMode)))
  (Variables|/Game/GameModes/BP_GameMode.BP_GameMode_C|SetbSpawnEnemies _asbp_game_mode false))

(event Custom|Client_OpenUI
  (Utilities|FlowControl|Sequence
    (:then_0
      (Development|PrintText (Utilities|Text|FormatText "Controlled Pawn: {Pawn}" (Utilities|GetDisplayName (Pawn|GetControlledPawn)))))
    (:then_1
      (bind _returnvalue (UserInterface|CreateWidget "/Game/UI/WBP_Game.WBP_Game_C" self))
      (UserInterface|Viewport|AddtoViewport _returnvalue 0))))

(event Input|EnhancedActionEvents|EnhancedInputActionIA_Move
  (params (ActionValue :type Vector%202D%20Structure) (ElapsedSeconds :type Float%20%28double-precision%29) (TriggeredSeconds :type Float%20%28double-precision%29) (InputAction :type Input%20Action%20Object%20Reference :default "/Game/Input/IA_Move.IA_Move"))
  (bind _asplayer (Variables|Default|GetAsPlayer)
    (:then
      (Default|Move _asplayer (.x ActionValue) (.y ActionValue)))
    (:else)))

(event Input|EnhancedActionEvents|EnhancedInputActionIA_Shoot
  (params (ActionValue :type Boolean) (ElapsedSeconds :type Float%20%28double-precision%29) (TriggeredSeconds :type Float%20%28double-precision%29) (InputAction :type Input%20Action%20Object%20Reference :default "/Game/Input/IA_Shoot.IA_Shoot"))
  (if ActionValue
    (bind _asplayer (Variables|Default|GetAsPlayer)
      (:then
        (Default|ServerShootBullet _asplayer "0, 0, 0"))
      (:else))))

(event EventBeginPlay
  (if (Pawn|IsLocalPlayerController)
    (Input|AddMappingContext (PlayerController|LocalPlayerSubsystems|GetEnhancedInputLocalPlayerSubsystem) "/Game/Input/IMC_Main.IMC_Main" 0 "(bIgnoreAllPressedKeysUntilRelease=True,bForceImmediately=False,bNotifyUserSettings=False)")
    (bind _outactors (Actor|GetAllActorsOfClass "/Game/Camera/BP_CameraActor.BP_CameraActor_C"))
    (if (Utilities|Array|IsNotEmpty _outactors)
      (Game|Player|SetViewTargetwithBlend (Utilities|Array|Get(acopy) _outactors) 0.0 "VTBlend_Linear" 0.0 false))))

(event EventPossess
  (params (PossessedPawn :type Pawn%20Object%20Reference))
  (bind _asbp_player (Utilities|Casting|CastToBP_Player PossessedPawn))
  (Variables|Default|SetAsPlayer _asbp_player)
  (Utilities|FlowControl|Delay 0.2)
  (CallFunction|ClientOpenUI)
  (Development|PrintText (Utilities|Text|FormatText "Controlled Pawn: {Pawn}" (Utilities|GetDisplayName (Pawn|GetControlledPawn)))))

(event Input|KeyboardEvents|1
  (params (Key :type Key%20Structure :default "None"))
  (:Pressed
    (CallFunction|ServerStopSpawnEnemy)))

(fn ConstructionScript)