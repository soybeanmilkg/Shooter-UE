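; Base pickup actor that drifts horizontally in a random direction at a random speed and expires after a random lifespan.
; On the server, box overlap with a BP_Player calls ApplyPickup, an empty hook, then multicasts and destroys the actor.
; Overlap with a "Border"-tagged actor reflects its velocity off the hit normal.
; The multicast plays the pickup sound in 2D only on machines without authority.
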(event OnComponentBeginOverlap(Box)
  (params (OverlappedComponent :type Primitive%20Component%20Object%20Reference) (OtherActor :type Actor%20Object%20Reference) (OtherComp :type Primitive%20Component%20Object%20Reference) (OtherBodyIndex :type Integer) (bFromSweep :type Boolean) (SweepResult :type Hit%20Result%20Structure%20%28by%20ref%29))
  (Networking|SwitchHasAuthority
    (:Authority
      (bind _asbp_player (Utilities|Casting|CastToBP_Player OtherActor)
        (:then
          (CallFunction|ApplyPickup _asbp_player)
          (CallFunction|MulticastonPickup)
          (Actor|DestroyActor))
        (:CastFailed
          (if (Actor|ActorHasTag OtherActor "Border")
            (Variables|/Script/Engine.MovementComponent|SetVelocity (Variables|Default|GetProjectileMovement) (Math|Vector|GetReflectionVector (Variables|/Script/Engine.MovementComponent|GetVelocity (Variables|Default|GetProjectileMovement)) (.Normal (Collision|BreakHitResult SweepResult))))))))))

(event Custom|Multicast_OnPickup
  (Networking|SwitchHasAuthority
    (:Remote
      (Audio|PlaySound2D (Variables|Default|GetPickupSound) 1.0 1.0 0.0 0 0))))

(event EventBeginPlay
  (Networking|SwitchHasAuthority
    (:Authority
      (Variables|/Script/Engine.ProjectileMovementComponent|SetMaxSpeed (Variables|Default|GetProjectileMovement) (Math|Random|RandomFloatinRange 4e+02 6e+02))
      (Variables|/Script/Engine.MovementComponent|SetVelocity (Variables|Default|GetProjectileMovement) (* (Math|Vector|RotateVectorAroundAxis "1.000000,0.000000,0.000000" (Math|Random|RandomFloatinRange 0.0 3.6e+02) "0.000000,0.000000,1.000000") (Variables|/Script/Engine.ProjectileMovementComponent|GetMaxSpeed (Variables|Default|GetProjectileMovement))))
      (Actor|SetLifeSpan (Math|Random|RandomFloatinRange 1e+01 15.0)))))

(fn ConstructionScript)

(fn ApplyPickup
  (params (InPlayer :type BP%20Player%20Object%20Reference)))